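; BP_Mikan is an actor with cursor-targeted, click-to-move controls, apparently the player's character.
; Every tick it traces under the cursor on the Visibility channel and places MouseTarget, a decal marker, at the hit, aligned to the surface normal.
; MoveToLocation, not called within this Blueprint, sends the PC_Character controller to a given hit via SimpleMoveToLocation if it is at least MinClickDistance away, with debug prints.
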(event EventTick
  (params (DeltaSeconds :type Float%20%28single-precision%29))
  (bind _returnvalue (Game|GetPlayerController 0))
  (bind _hitresult (Game|Player|GetHitResultUnderCursorbyChannel _returnvalue "TraceTypeQuery1" true))
  (bind (_bblockinghit _binitialoverlap _time _location _impactpoint _normal _impactnormal) (Collision|BreakHitResult _hitresult))
  ;[1 1 1] Get Mouse Pos. in World w/ Ray Cast
  ;[1 1 1] Apply Decal to Target Location
  (Transformation|SetWorldLocationAndRotation (Variables|Default|GetMouseTarget) _location (Math|Rotator|MakeRotationfromAxes _impactnormal "0, 0, 0" "0, 0, 0") false false))

(fn ConstructionScript)

(fn MovetoLocation
  (params (Hit :type Hit%20Result%20Structure))
  (bind _location (Collision|BreakHitResult Hit))
  (Development|PrintString "called")
  (if (>= (Math|Vector|VectorLength (- (Transformation|GetActorLocation self) _location)) (LocalVariables|GetMin_Click_Distance))
    (bind _aspc_character (Utilities|Casting|CastToPC_Character (Game|GetPlayerController 0)))
    (AI|Navigation|SimpleMovetoLocation _aspc_character _location)
    (Development|PrintString "Hello")))